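; BP_MCActorBase is a base grid actor Blueprint that provides an overhead-style widget hookup and visual damage feedback.
; On BeginPlay it caches the mesh's default material and initializes its WBP_MCActor widget with itself.
; OnDamage swaps the mesh to a yellow hex material, and a timer lasting half the MCWorldSettings world time step restores the cached material.
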(event Custom|OnDamageEffectFinished
  (Rendering|Material|SetMaterial (Variables|Character|GetMesh) 0 (Variables|Default|GetCachedMaterial)))

(event EventBeginPlay
  (Utilities|FlowControl|Sequence
    (:then_0
      ;[0.15 0.15 0.15 0.5] Cache default material
      (Variables|Default|SetCachedMaterial (Rendering|Material|GetMaterial (Variables|Character|GetMesh) 0)))
    (:then_1
      ;[0.15 0.15 0.15 0.5] Init Widget
      (bind _aswbp_mcactor (Utilities|Casting|CastToWBP_MCActor (UserInterface|GetWidget (Variables|Default|GetWidget))))
      (Default|Init _aswbp_mcactor (Utilities|ResolveSoftReference self)))))

(event EventOnDamage
  (Rendering|Material|SetMaterial (Variables|Character|GetMesh) 0 "/Game/Materials/MI_Hex_Yellow.MI_Hex_Yellow")
  (bind _returnvalue (Class|World|GetWorldSettings (Class|MCActorBase|GetWorld)))
  (bind _asmcworld_settings (Utilities|Casting|CastToMCWorldSettings _returnvalue))
  (Utilities|Time|SetTimerbyEvent (delegate Custom|OnDamageEffectFinished) (/ (Variables|/Script/Microcosm.MCWorldSettings|GetWorldTimeStep _asmcworld_settings) 2.0)))

(fn ConstructionScript)